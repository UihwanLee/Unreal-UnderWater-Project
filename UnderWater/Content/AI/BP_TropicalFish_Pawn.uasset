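; BP_TropicalFish_Pawn is a tropical fish pawn that swims in a straight line until it is killed.
; Each tick it advances a stored target location along its forward vector by a fixed, frame-rate-dependent step and moves there.
; Its look-at rotation uses identical start and target points, so it resolves to zero and the fish heads along world X.
; Damage above a small threshold spawns BP_TropicalFish_Dead at that location and destroys the pawn.
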(event `self.ReceiveBeginPlay`
  (set `self.TargetLocation` (`self.K2_GetActorLocation`)))

(event `self.ReceiveTick`
  (params (DeltaSeconds :type "Float (single-precision)"))
  (bind _targetlocation (`self.TargetLocation`))
  (bind _output_get (set `self.TargetLocation` (+ _targetlocation (* (`self.GetActorForwardVector`) 1.01))))
  (`self.K2_SetActorLocationAndRotation` _output_get (`KismetMathLibrary.FindLookAtRotation` _targetlocation _output_get)))

(event `self.ReceiveAnyDamage`
  (params (Damage :type "Float (single-precision)") (DamageType :type "DamageType Object Reference") (InstigatedBy :type "Controller Object Reference") (DamageCauser :type "Actor Object Reference"))
  (if (> Damage 10.0)
    (`|SpawnActorFromClass` "/Game/AI/BP_TropicalFish_Dead.BP_TropicalFish_Dead_C" (`KismetMathLibrary.Conv_VectorToTransform` (`self.TargetLocation`)) "Undefined" "MultiplyWithRoot" null null)
    (`self.K2_DestroyActor`)))

(fn `UserConstructionScript`)