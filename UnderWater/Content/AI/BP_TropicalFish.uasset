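; BP_TropicalFish is a fish actor that drifts along the world X axis.
; It stores its spawn location, then each Tick adds a random Min–Max X offset, unscaled by delta time, and moves there.
; Its look-at rotation uses the target as both start and end, so it gives no real heading; a rotation interpolation node is left unused.
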(event `self.ReceiveBeginPlay`
  (set `self.TargetLocation` (`self.K2_GetActorLocation`)))

(event `self.ReceiveTick`
  (params (DeltaSeconds :type "Float (single-precision)"))
  (bind _targetlocation (`self.TargetLocation`))
  (bind _output_get (set `self.TargetLocation` (+ _targetlocation (`KismetMathLibrary.MakeVector` (`KismetMathLibrary.RandomFloatInRange` (`self.Min`) (`self.Max`))))))
  (`self.K2_SetActorLocationAndRotation` _output_get (`KismetMathLibrary.FindLookAtRotation` _targetlocation _output_get)))

(fn `UserConstructionScript`)