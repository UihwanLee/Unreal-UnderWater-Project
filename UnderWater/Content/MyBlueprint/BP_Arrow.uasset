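; BP_Arrow is an arrow projectile that is launched through a Fire event with a given velocity.
; Collision is off at BeginPlay, and Fire hands the static mesh to the ProjectileMovement component and activates it.
; After a short delay, Fire re-enables actor collision and sets the mesh to block all dynamic, so the launch itself is collision-free.
; The Grab function is a stub that always returns false.
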(event `self.ReceiveBeginPlay`
  (`self.SetActorEnableCollision` false))

(event `/Game/MyBlueprint/Handle.Fire`
  (params (Velocity :type "Vector Structure"))
  (bind _projectilemovement (`self.ProjectileMovement`))
  (set `MovementComponent.Velocity` Velocity _projectilemovement)
  (`MovementComponent.SetUpdatedComponent` _projectilemovement (`self.StaticMesh`))
  (`ActorComponent.Activate` _projectilemovement true)
  (`KismetSystemLibrary.Delay` 0.2)
  (`self.SetActorEnableCollision` true)
  (`PrimitiveComponent.SetCollisionProfileName` (`self.StaticMesh`) "BlockAllDynamic" true))

(fn `Grab`
  (returns (`Is Grab ?` :type Boolean))
  (return false))

(fn `UserConstructionScript`)